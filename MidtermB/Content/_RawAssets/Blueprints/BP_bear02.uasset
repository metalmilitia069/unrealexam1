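; BP_bear02 is a damageable bear actor with a static mesh that flashes when hit and is destroyed when its health runs out.
; Each Hit event decrements Hp and destroys the actor when it equals exactly zero.
; Otherwise, it briefly raises the materials' Emissive scalar parameter, then resets it after a short Delay.
; A leftover FlipFlop branch is never executed.
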(event `self.ReceiveHit`
  (params (MyComp :type "PrimitiveComponent Object Reference") (Other :type "Actor Object Reference") (OtherComp :type "PrimitiveComponent Object Reference") (bSelfMoved :type Boolean) (HitLocation :type "Vector Structure") (HitNormal :type "Vector Structure") (NormalImpulse :type "Vector Structure") (Hit :type "HitResult Structure (by ref)"))
  (bind _staticmeshcomponent0 (`self.StaticMeshComponent0`))
  (set `self.hp` (- (`self.hp`) 1))
  (bind _output_get (set `self.IsDead` (== (`self.hp`) 0)))
  (if _output_get
    (`self.K2_DestroyActor`)
    (else
      (`MeshComponent.SetScalarParameterValueOnMaterials` _staticmeshcomponent0 "Emissive" 1.0)
      (`KismetSystemLibrary.Delay` 0.2)
      (`MeshComponent.SetScalarParameterValueOnMaterials` _staticmeshcomponent0 "Emissive" 0.0))))

(fn `UserConstructionScript`)